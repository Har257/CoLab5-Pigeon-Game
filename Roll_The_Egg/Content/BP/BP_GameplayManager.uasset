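; Gameplay manager for an egg-rolling level that switches between an edit camera mode and an egg roll mode.
; Space or left click drives the swaps, using timelines to glide the edit camera, switching possession and input mode, and resetting the egg and stars.
; It also owns the overlay, fail and victory widgets.
; Winning saves best stars and unlocks the next level in BP_GIManager through hard-coded level-name checks.
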(event `Overlay menu`
  ; Initilises overlay menu
  (bind _returnvalue (`|CreateWidget` "/Game/BP/UI/WBP_ScreenOverlay.WBP_ScreenOverlay_C" (`GameplayStatics.GetPlayerController` 0)))
  (set `self.OverlayUI` _returnvalue)
  (`UserWidget.AddToViewport` _returnvalue 0)
  (if (not (`self.StartEgg`))
    (`/Game/BP/UI/WBP_ScreenOverlay.ShowRoll` (`self.OverlayUI`))))

(event `EggDied`
  ; Fail screen open and close
  (if (not (`self.MenuActive`))
    (set `self.MenuActive` true)
    (`KismetSystemLibrary.Delay` 0.2)
    (bind _returnvalue (`|CreateWidget` "/Game/BP/UI/WBP_FailScreen.WBP_FailScreen_C" (`GameplayStatics.GetPlayerController` 0)))
    (`UserWidget.AddToViewport` _returnvalue 0)))

(event `FailUIAniUpFin`
  (bind _returnvalue (`GameplayStatics.GetPlayerController` 0))
  ; Fail screen open and close
  (`WidgetBlueprintLibrary.SetInputMode_UIOnlyEx` _returnvalue (stale `EggDied` _returnvalue))
  (set `PlayerController.bShowMouseCursor` true _returnvalue))

(event `CloseFailScreen`
  ; Fail screen open and close
  (`GameplayStatics.SetGlobalTimeDilation` 1.0)
  (`Widget.RemoveFromParent` (stale `EggDied` _returnvalue))
  (`self.SetEditMode`)
  (set `self.MenuActive` false))

(event `UpdateMaxStarInLevel`
  (bind _gameinstance (`self.GameInstance`))
  (bind _starscollected (`self.StarsCollected`))
  (bind _gameinstance_2 (`self.GameInstance`))
  (bind _gameinstance_3 (`self.GameInstance`))
  (bind _starscollected_2 (`self.StarsCollected`))
  ; When the Egg has entered the nest, and opende the win screen the Singelton is updated with the unlcok and most stars achived
  (bind _returnvalue (`GameplayStatics.GetCurrentLevelName` true))
  (if (`KismetStringLibrary.EqualEqual_StrStr` _returnvalue "00_Level")
    (set `/Game/BP/BP_GIManager.L_Locked_0` false _gameinstance)
    (if (> _starscollected_2 (`/Game/BP/BP_GIManager.L_Stars` _gameinstance_3))
      (set `/Game/BP/BP_GIManager.L_Stars` _starscollected _gameinstance_2))
    (elif (`KismetStringLibrary.EqualEqual_StrStr` _returnvalue "0_Level")
      (set `/Game/BP/BP_GIManager.L_Locked_1` false _gameinstance)
      (if (> _starscollected_2 (`/Game/BP/BP_GIManager.L_Stars_0` _gameinstance_3))
        (set `/Game/BP/BP_GIManager.L_Stars_0` _starscollected _gameinstance_2))
      (elif (`KismetStringLibrary.EqualEqual_StrStr` _returnvalue "1_Level")
        (set `/Game/BP/BP_GIManager.L_Locked_2` false _gameinstance)
        (if (> _starscollected_2 (`/Game/BP/BP_GIManager.L_Stars_1` _gameinstance_3))
          (set `/Game/BP/BP_GIManager.L_Stars_1` _starscollected _gameinstance_2))
        (elif (`KismetStringLibrary.EqualEqual_StrStr` _returnvalue "2_Level")
          (if (> _starscollected_2 (`/Game/BP/BP_GIManager.L_Stars_2` _gameinstance_3))
            (set `/Game/BP/BP_GIManager.L_Stars_2` _starscollected _gameinstance_2)))))))

(event `EggHome`
  ; Win screen open and close
  (if (not (`self.MenuActive`))
    (set `self.MenuActive` true)
    (set `self.StarsCollected` (`/Game/Egg/BP_EggPlayer.Score` (`self.BP_EggPlayer`)))
    (`self.UpdateMaxStarInLevel`)
    (bind _returnvalue (`|CreateWidget` "/Game/BP/UI/WBP_VictoryScreen.WBP_VictoryScreen_C" (`GameplayStatics.GetPlayerController` 0)))
    (`UserWidget.AddToViewport` _returnvalue 0)))

(event `VictoryUIAniUp`
  (bind _returnvalue (`GameplayStatics.GetPlayerController` 0))
  ; Win screen open and close
  (`WidgetBlueprintLibrary.SetInputMode_UIOnlyEx` _returnvalue (stale `EggHome` _returnvalue))
  (set `PlayerController.bShowMouseCursor` true _returnvalue))

(event `CloseWinScreen`
  ; Win screen open and close
  (`Widget.RemoveFromParent` (stale `EggHome` _returnvalue))
  (`self.SetEditMode`)
  (set `self.MenuActive` false))

(event `ModeGameOnlyHideCurrsor`
  (bind _returnvalue (`GameplayStatics.GetPlayerController` 0))
  ; Controls possession and mouse visibility for the different modes
  (`WidgetBlueprintLibrary.SetInputMode_GameOnly` _returnvalue)
  (set `PlayerController.bShowMouseCursor` false _returnvalue))

(event `self.ReceiveBeginPlay`
  ; Gets all needed refs and sets player in selected mode
  (bind _asbp_gimanager (cast `/Game/BP/BP_GIManager` (`GameplayStatics.GetGameInstance`)))
  (set `self.GameInstance` _asbp_gimanager)
  (bind _returnvalue (`GameplayStatics.GetActorOfClass` "/Game/Egg/BP_EggPlayer.BP_EggPlayer_C"))
  (set `self.BP_EggPlayer` _returnvalue)
  (bind _returnvalue_2 (`GameplayStatics.GetActorOfClass` "/Game/BP/BP_EditCamPlayer.BP_EditCamPlayer_C"))
  (set `self.BP_EditCam` _returnvalue_2)
  (bind _outactors (`GameplayStatics.GetAllActorsOfClass` "/Game/BP/BP_StarObjective.BP_StarObjective_C"))
  (set `self.AllLevelStars` _outactors)
  (set `self.EggCamDefultLocation` (`SceneComponent.K2_GetComponentLocation` (`/Game/Egg/BP_EggPlayer.EggCam` (`self.BP_EggPlayer`))))
  (set `self.EditCamDefultStartLocatiom` (`SceneComponent.K2_GetComponentLocation` (`/Game/BP/BP_EditCamPlayer.Camera` (`self.BP_EditCam`))))
  (`self.EnableInput` (`GameplayStatics.GetPlayerController` 0))
  (`self.Overlay menu`)
  (if (`self.StartEgg`)
    (`self.EggPossess`)
    (else
      (`self.EditCamPossess`))))

(event `EggPossess`
  ; Controls possession and mouse visibility for the different modes
  (`Controller.Possess` (`GameplayStatics.GetPlayerController` 0) (`self.BP_EggPlayer`))
  (set `/Game/BP/BP_GIManager.IsInEggMode` true (`self.GameInstance`))
  (`self.ModeGameOnlyHideCurrsor`))

(event `Key|LeftMouseButton` :consume false :overrideparent false
  (params (Key :type "Key Structure"))
  ; Stops the current roll when clicking
  (:`Pressed`
    (if (`self.MenuActive`)
      _
      (elif (`self.SwappingMode`)
        _
        (elif (`/Game/BP/BP_GIManager.IsInEggMode` (`self.GameInstance`))
          (if (`/Game/Egg/BP_EggPlayer.IsRolling` (`self.BP_EggPlayer`))
            (`self.Start/StopRoll`)))))))

(event `EditCamPossess`
  (bind _returnvalue (`GameplayStatics.GetPlayerController` 0))
  (bind _bp_editcam (`self.BP_EditCam`))
  ; Controls possession and mouse visibility for the different modes
  (`Controller.Possess` (`GameplayStatics.GetPlayerController` 0) _bp_editcam)
  (set `/Game/BP/BP_GIManager.IsInEggMode` false (`self.GameInstance`))
  (`self.EnableInput` _bp_editcam _returnvalue)
  (`WidgetBlueprintLibrary.SetInputMode_GameAndUIEx` _returnvalue (`self.OverlayUI`) "DoNotLock" false)
  (set `PlayerController.bShowMouseCursor` true _returnvalue))

(event `SetEditMode`
  (bind _bp_editcam (`self.BP_EditCam`))
  (bind _bp_eggplayer (`self.BP_EggPlayer`))
  (bind _rootcomponent (`Actor.RootComponent` (`self.BP_EditCam`)))
  (bind _returnvalue (`SceneComponent.K2_GetComponentLocation` (`/Game/Egg/BP_EggPlayer.EggCam` _bp_eggplayer)))
  ; Handles the animation and transition steps, swapping between the edit and egg modes
  (`/Game/BP/UI/WBP_ScreenOverlay.ShowRoll` (`self.OverlayUI`) :!label _label)
  (set `self.SwappingMode` true)
  (if (`/Game/Egg/BP_EggPlayer.IsRolling` _bp_eggplayer)
    (`SceneComponent.K2_SetWorldLocation` _rootcomponent _returnvalue false false)
    (`/Game/Egg/BP_EggPlayer.EggReset` _bp_eggplayer)
    (`/Game/BP/BP_StarObjective.ReloadStarsCheck` (`self.AllLevelStars`))
    (else
      (`SceneComponent.K2_SetWorldLocation` _rootcomponent _returnvalue false false)))
  (if (`self.RetunEditCamToStartLocation`)
    (set `self.EditCamCurrentLocation` (`SceneComponent.K2_GetComponentLocation` (`/Game/BP/BP_EditCamPlayer.Camera` (`self.BP_EditCam`))))
    (`Controller.Possess` (`GameplayStatics.GetPlayerController` 0) _bp_editcam)
    (bind (_direction _editcamtoeggcam) (`Timeline|Timeline_0` :!via `PlayFromStart`)
      (:`Update`
        (`SceneComponent.K2_SetWorldLocation` (`Actor.RootComponent` _bp_editcam) (`KismetMathLibrary.VLerp` (`self.EditCamCurrentLocation`) (`self.EditCamDefultStartLocatiom`) _editcamtoeggcam) false false))
      (:`Finished`
        (`self.EditCamPossess`)
        (set `self.SwappingMode` false)))
    (else
      (`self.EditCamPossess`)
      (set `self.SwappingMode` false))))

(event `Start/StopRoll`
  (bind _returnvalue (`GameplayStatics.GetPlayerController` 0))
  (bind _bp_editcam (`self.BP_EditCam`))
  ; Handles the animation and transition steps, swapping between the edit and egg modes
  (if (`self.SwappingMode`) :!label _label_2
    _
    (elif (`/Game/BP/BP_GIManager.IsInEggMode` (`self.GameInstance`))
      (goto _label)
      (else
        (`/Game/BP/UI/WBP_ScreenOverlay.HideRoll` (`self.OverlayUI`))
        (`/Game/Egg/BP_EggPlayer.EggReset` (`self.BP_EggPlayer`))
        (`/Game/BP/BP_StarObjective.ReloadStarsCheck` (`self.AllLevelStars`))
        (set `self.SwappingMode` true)
        (`/Game/BP/BP_EditCamPlayer.Forced Drop` _bp_editcam)
        (`self.DisableInput` _bp_editcam null)
        (set `self.EditCamCurrentLocation` (`SceneComponent.K2_GetComponentLocation` (`/Game/BP/BP_EditCamPlayer.Camera` _bp_editcam)))
        (`WidgetBlueprintLibrary.SetInputMode_GameOnly` _returnvalue)
        (set `PlayerController.bShowMouseCursor` false _returnvalue)
        (bind (_direction _editcamtoeggcam) (`Timeline|Timeline` :!via `PlayFromStart`)
          (:`Update`
            (`SceneComponent.K2_SetWorldLocation` (`Actor.RootComponent` (`self.BP_EditCam`)) (`KismetMathLibrary.VLerp` (`self.EditCamCurrentLocation`) (`self.EggCamDefultLocation`) _editcamtoeggcam) false false))
          (:`Finished`
            (`self.EggPossess`)
            (set `self.SwappingMode` false)
            (`/Game/Egg/BP_EggPlayer.StartRoll` (`self.BP_EggPlayer`))))))))

(event `Key|SpaceBar` :consume false :overrideparent false
  (params (Key :type "Key Structure"))
  ; Handles the animation and transition steps, swapping between the edit and egg modes
  (:`Pressed`
    (goto _label_2)))

(fn `UserConstructionScript`)