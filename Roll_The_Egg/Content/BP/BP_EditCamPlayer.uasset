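; Edit-mode player pawn for panning and zooming the camera and placing BP_MoveableObjectBase objects with the mouse.
; Left-drag grabs the object under the cursor and grid-snaps it in the Y/Z plane, while the wheel rotates it in 45-degree steps.
; Moves and rotations go to an overlap-test pivot first, reaching the object only when clear.
; Right-drag pans, the wheel otherwise zooms, and StoppedEditMode disables input and force-drops the object.
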(event `RotateToCheck`
  (bind _selectedobject (`self.SelectedObject`))
  (bind _rootcomponent (`Actor.RootComponent` _selectedobject))
  ; Checks the tester for the rotation and if viable updates the rotations to match
  (if (not (`/Game/BP/Draggables/BP_MoveableObjectBase.IsOverlapping` (`self.SelectedObject`)))
    (`SceneComponent.K2_SetWorldRotation` _rootcomponent (`SceneComponent.K2_GetComponentRotation` (`/Game/BP/Draggables/BP_MoveableObjectBase.PivotPointOverlapTest` (`self.SelectedObject`))) false false)
    (`SceneComponent.K2_SetWorldRotation` (`/Game/BP/Draggables/BP_MoveableObjectBase.PivotPointOverlapTest` _selectedobject) (`SceneComponent.K2_GetComponentRotation` _rootcomponent) false false)
    (set `self.TryingRotate` false)))

(event `self.ReceiveBeginPlay`
  ; Gets ref to Singelton and sets capture mode
  (bind _asbp_gimanager (cast `/Game/BP/BP_GIManager` (`GameplayStatics.GetGameInstance`)))
  (set `self.GameInstance` _asbp_gimanager)
  (`GameplayStatics.SetViewportMouseCaptureMode` "CaptureDuringMouseDown"))

(event `StoppedEditMode`
  ; Called by other scripts to interupt object drag
  (`self.DisableInput` (`GameplayStatics.GetPlayerController` 0))
  (`self.Forced Drop`))

(event `Key|MouseScrollUp` :consume false :overrideparent false
  (params (Key :type "Key Structure"))
  ; Checks the tester for the rotation and if viable updates the rotations to match
  (:`Pressed`
    (if (`self.LmbHeld`)
      (if (`self.ObjectSelected`)
        (if (`/Game/BP/Draggables/BP_MoveableObjectBase.CanRotate` (`self.SelectedObject`))
          (set `self.TryingRotate` true)
          (`SceneComponent.K2_SetWorldRotation` (`/Game/BP/Draggables/BP_MoveableObjectBase.PivotPointOverlapTest` (`self.SelectedObject`)) (`KismetMathLibrary.MakeRotator` (+ (.roll (`SceneComponent.K2_GetComponentRotation` (`/Game/BP/Draggables/BP_MoveableObjectBase.PivotPointOverlapTest` (`self.SelectedObject`)))) 45.0) (.pitch (`SceneComponent.K2_GetComponentRotation` (`/Game/BP/Draggables/BP_MoveableObjectBase.PivotPointOverlapTest` (`self.SelectedObject`)))) (.yaw (`SceneComponent.K2_GetComponentRotation` (`/Game/BP/Draggables/BP_MoveableObjectBase.PivotPointOverlapTest` (`self.SelectedObject`))))) false false))))))

(event `Key|MouseScrollDown` :consume false :overrideparent false
  (params (Key :type "Key Structure"))
  ; Checks the tester for the rotation and if viable updates the rotations to match
  (:`Pressed`
    (if (`self.LmbHeld`)
      (if (`self.ObjectSelected`)
        (if (`/Game/BP/Draggables/BP_MoveableObjectBase.CanRotate` (`self.SelectedObject`))
          (set `self.TryingRotate` true)
          (`SceneComponent.K2_SetWorldRotation` (`/Game/BP/Draggables/BP_MoveableObjectBase.PivotPointOverlapTest` (`self.SelectedObject`)) (`KismetMathLibrary.MakeRotator` (- (.roll (`SceneComponent.K2_GetComponentRotation` (`/Game/BP/Draggables/BP_MoveableObjectBase.PivotPointOverlapTest` (`self.SelectedObject`)))) 45.0) (.pitch (`SceneComponent.K2_GetComponentRotation` (`/Game/BP/Draggables/BP_MoveableObjectBase.PivotPointOverlapTest` (`self.SelectedObject`)))) (.yaw (`SceneComponent.K2_GetComponentRotation` (`/Game/BP/Draggables/BP_MoveableObjectBase.PivotPointOverlapTest` (`self.SelectedObject`))))) false false))))))

(event `Key|LeftMouseButton` :consume false :overrideparent false
  (params (Key :type "Key Structure"))
  (bind _selectedobject (`self.SelectedObject`))
  (bind _defaultsceneroot (`/Game/BP/Draggables/BP_MoveableObjectBase.DefaultSceneRoot` (`self.SelectedObject`)))
  ; Handels drag movement
  (:`Pressed`
    (set `self.LmbHeld` true)
    (bind _asbp_moveable_object_base (cast `/Game/BP/Draggables/BP_MoveableObjectBase` (`.HitActor` (`GameplayStatics.BreakHitResult` (`PlayerController.GetHitResultUnderCursorByChannel` (`GameplayStatics.GetPlayerController` 0) "TraceTypeQuery2" true)))))
    (set `self.SelectedObject` _asbp_moveable_object_base)
    (set `self.ObjectSelected` true)
    (`/Game/BP/Draggables/BP_MoveableObjectBase.ObjectGrabbed` _selectedobject))
  (:`Released`
    (set `self.LmbHeld` false :!label _label)
    (if (`self.ObjectSelected`)
      (`SceneComponent.K2_SetWorldLocationAndRotation` (`/Game/BP/Draggables/BP_MoveableObjectBase.PivotPointOverlapTest` (`self.SelectedObject`)) (`SceneComponent.K2_GetComponentLocation` _defaultsceneroot) (`SceneComponent.K2_GetComponentRotation` _defaultsceneroot) false false)
      (set `self.ObjectSelected` false)
      (`/Game/BP/Draggables/BP_MoveableObjectBase.ObjectDropped` _selectedobject)
      (set `self.SelectedObject` null))))

(event `Forced Drop`
  ; Handels drag movement
  (goto _label))

(event `Key|MouseScrollUp` :consume false :overrideparent false
  (params (Key :type "Key Structure"))
  ; Camera Movement
  ;; Moves the camera forward/back on the scroll
  (:`Pressed`
    (if (not (`self.LmbHeld`))
      (`self.AddMovementInput` (`SceneComponent.GetForwardVector` (`self.Camera`))))))

(event `Key|RightMouseButton` :consume false :overrideparent false
  (params (Key :type "Key Structure"))
  (bind (_locationx _locationy) (`WidgetLayoutLibrary.GetMousePositionScaledByDPI` (`GameplayStatics.GetPlayerController` 0)))
  ; Camera Movement
  ;; Initilises the camera drag movement
  (:`Pressed`
    (set `self.MbDrag` true)
    (set `self.LastMousePos` (`KismetMathLibrary.MakeVector2D` _locationx _locationy)))
  (:`Released`
    (set `self.MbDrag` false)))

(event `DraggingObject`
  (bind _selectedobject (`self.SelectedObject`))
  (bind _selectedobject_2 (`self.SelectedObject`))
  ; Handels drag movement
  ;; Moves the draggable objects testing box and then if theres space move the root and test that avaidable space
  (`/Engine/EditorBlueprintResources/StandardMacros.DoOnce` false :!label _label_2
    (:`Completed`
      (bind _output_get (set `self.TestLocation` (`KismetMathLibrary.MakeVector` 550.0 (`KismetMathLibrary.GridSnap_Float` (.y (`.ImpactPoint` (`GameplayStatics.BreakHitResult` (`PlayerController.GetHitResultUnderCursorByChannel` (`GameplayStatics.GetPlayerController` 0) "TraceTypeQuery2" true)))) 10.0) (`KismetMathLibrary.GridSnap_Float` (.z (`.ImpactPoint` (`GameplayStatics.BreakHitResult` (`PlayerController.GetHitResultUnderCursorByChannel` (`GameplayStatics.GetPlayerController` 0) "TraceTypeQuery2" true)))) 10.0))))
      (`SceneComponent.K2_SetWorldLocation` (`/Game/BP/Draggables/BP_MoveableObjectBase.PivotPointOverlapTest` _selectedobject_2) _output_get false false)
      (if (`/Game/BP/Draggables/BP_MoveableObjectBase.IsOverlapping` _selectedobject_2)
        (`self.FinishedDragCycle`)
        (else
          (bind _output_get_2 (set `self.ViableLocation` (`self.TestLocation`)))
          (`SceneComponent.K2_SetRelativeLocation` (`/Game/BP/Draggables/BP_MoveableObjectBase.PivotPointOverlapTest` _selectedobject) (0.0 0.0 0.0) false false)
          (`SceneComponent.K2_SetWorldLocation` (`/Game/BP/Draggables/BP_MoveableObjectBase.DefaultSceneRoot` _selectedobject) _output_get_2 false false)
          (`self.FinishedDragCycle`))))))

(event `FinishedDragCycle`
  ; Handels drag movement
  ;; Moves the draggable objects testing box and then if theres space move the root and test that avaidable space
  (goto _label_2 :!via `Reset`))

(event `Key|MouseScrollDown` :consume false :overrideparent false
  (params (Key :type "Key Structure"))
  ; Camera Movement
  ;; Moves the camera forward/back on the scroll
  (:`Pressed`
    (if (not (`self.LmbHeld`))
      (`self.AddMovementInput` (* (`SceneComponent.GetForwardVector` (`self.Camera`)) -1)))))

(event `DragMoveUpdate`
  (bind (_locationx _locationy) (`WidgetLayoutLibrary.GetMousePositionScaledByDPI` (`GameplayStatics.GetPlayerController` 0)))
  (bind (_locationx_2 _locationy_2) (`WidgetLayoutLibrary.GetMousePositionScaledByDPI` (`GameplayStatics.GetPlayerController` 0)))
  (bind _returnvalue (`KismetMathLibrary.MakeVector2D` _locationx_2 _locationy_2))
  ; Camera Movement
  ;; Drag camera movement
  (`self.AddMovementInput` (`KismetMathLibrary.Normal` (`KismetMathLibrary.MakeVector` 0.0 (`KismetMathLibrary.BreakVector2D` (- (`self.LastMousePos`) _returnvalue)) (`.Y` (`KismetMathLibrary.BreakVector2D` (- _returnvalue (`self.LastMousePos`)))))) 0.5)
  (set `self.LastMousePos` (`KismetMathLibrary.MakeVector2D` _locationx _locationy)))

(event `self.ReceiveTick`
  (params (DeltaSeconds :type "Float (single-precision)"))
  (bind _selectedobject (`self.SelectedObject`))
  ; Continuos update for move, drag and rotate attempts by the player
  (if (`self.MbDrag`)
    (`self.DragMoveUpdate`)
    (elif (`self.ObjectSelected`)
      (if (`/Game/BP/Draggables/BP_MoveableObjectBase.CanMove` _selectedobject)
        (`self.DraggingObject`))
      (if (`/Game/BP/Draggables/BP_MoveableObjectBase.CanRotate` _selectedobject)
        (if (`/Game/BP/Draggables/BP_MoveableObjectBase.CanMove` _selectedobject)
          (if (`self.TryingRotate`) :!label _label_3
            (`self.RotateToCheck`))
          (elif (`self.DropNoOverlapRotate`)
            (if (!= (`.HitActor` (`GameplayStatics.BreakHitResult` (`PlayerController.GetHitResultUnderCursorByChannel` (`GameplayStatics.GetPlayerController` 0) "TraceTypeQuery2" true))) (`self.SelectedObject`))
              (`self.Forced Drop`)
              (else
                (goto _label_3)))
            (else
              (goto _label_3))))))))

(fn `UserConstructionScript`)