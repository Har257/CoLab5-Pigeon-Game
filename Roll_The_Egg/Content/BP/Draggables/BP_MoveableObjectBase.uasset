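; Base Blueprint for moveable objects that shows a placement preview while grabbed and tracks whether the spot is blocked.
; ObjectGrabbed shows OverlapCheckMesh with the free-space material, and ObjectDropped hides it.
; Overlaps with components tagged "Blocking" set IsOverlapping and switch the mesh to the blocking material.
; On end overlap it rescans remaining overlaps, restoring the free-space material only when no blocker remains.
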(event `self.ReceiveBeginPlay`)

(event `self.OverlapCheckMesh.OnComponentBeginOverlap`
  (params (OverlappedComponent :type "PrimitiveComponent Object Reference") (OtherActor :type "Actor Object Reference") (OtherComp :type "PrimitiveComponent Object Reference") (OtherBodyIndex :type Integer) (bFromSweep :type Boolean) (SweepResult :type "HitResult Structure (by ref)"))
  ; Managers materiial changes and flags if its currently getting blocked or not
  (if (`ActorComponent.ComponentHasTag` OtherComp "Blocking")
    (set `self.IsOverlapping` true)
    (`PrimitiveComponent.SetMaterial` (`self.OverlapCheckMesh`) 0 "/Game/Materials/M_MovementPreviewBlocking.M_MovementPreviewBlocking")))

(event `self.OverlapCheckMesh.OnComponentEndOverlap`
  (params (OverlappedComponent :type "PrimitiveComponent Object Reference") (OtherActor :type "Actor Object Reference") (OtherComp :type "PrimitiveComponent Object Reference") (OtherBodyIndex :type Integer))
  ; Managers materiial changes and flags if its currently getting blocked or not
  (if (`ActorComponent.ComponentHasTag` OtherComp "Blocking")
    (set `self.IsOverlapping` false)
    (for _array_element (`PrimitiveComponent.GetOverlappingComponents` (`self.OverlapCheckMesh`))
      (if (`ActorComponent.ComponentHasTag` _array_element "Blocking")
        (set `self.IsOverlapping` true)))
    (if (not (`self.IsOverlapping`))
      (`PrimitiveComponent.SetMaterial` (`self.OverlapCheckMesh`) 0 "/Game/Materials/M_MovementPreviewSpace.M_MovementPreviewSpace"))))

(event `ObjectGrabbed`
  ; Managers materiial changes and flags if its currently getting blocked or not
  (`PrimitiveComponent.SetMaterial` (`self.OverlapCheckMesh`) 0 "/Game/Materials/M_MovementPreviewSpace.M_MovementPreviewSpace")
  (`SceneComponent.SetHiddenInGame` (`self.OverlapCheckMesh`) false false))

(event `ObjectDropped`
  ; Managers materiial changes and flags if its currently getting blocked or not
  (`SceneComponent.SetHiddenInGame` (`self.OverlapCheckMesh`) true false))

(fn `UserConstructionScript`)