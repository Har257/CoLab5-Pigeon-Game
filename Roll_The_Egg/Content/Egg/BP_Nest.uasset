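; BP_Nest is a goal actor that detects when a living egg player arrives home.
; It caches the BP_GameplayManager at BeginPlay.
; On overlap with a BP_EggPlayer whose health is above zero, it clears the rolling flag, zeroes the ball's linear velocity and calls EggHome on the manager.
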(event `self.ReceiveBeginPlay`
  (bind _returnvalue (`GameplayStatics.GetActorOfClass` "/Game/BP/BP_GameplayManager.BP_GameplayManager_C"))
  (set `self.BP_GameplayManager` _returnvalue))

(event `self.ReceiveActorBeginOverlap`
  (params (OtherActor :type "Actor Object Reference"))
  (bind _asbp_egg_player (cast `/Game/Egg/BP_EggPlayer` OtherActor))
  (if (> (`/Game/Egg/BP_EggPlayer.Health` _asbp_egg_player) 0.0)
    (set `/Game/Egg/BP_EggPlayer.IsRolling` false _asbp_egg_player)
    (`PrimitiveComponent.SetPhysicsLinearVelocity` (`/Game/Egg/BP_EggPlayer.RollingBall` _asbp_egg_player) (0.0 0.0 0.0) false "None")
    (`/Game/BP/BP_GameplayManager.EggHome` (`self.BP_GameplayManager`))))

(fn `UserConstructionScript`)