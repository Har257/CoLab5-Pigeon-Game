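; Player egg that rolls as a physics ball, can take damage and triggers game over when its health runs out.
; StartRoll or E enables physics and fires a one-time impulse; EggReset or T returns the ball to its cached start transform and re-arms the launch.
; Damage, also bound to N, lowers Health and swaps egg materials, then at zero hides the egg and shows the GameOverScreen widget with UI-only input.
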(event `self.ReceiveBeginPlay`
  (bind _rollingball (`self.RollingBall`))
  (bind _asbp_gimanager (cast `/Game/BP_GIManager` (`GameplayStatics.GetGameInstance`)))
  (set `self.GameInstance` _asbp_gimanager)
  (set `self.StartLocation` (`SceneComponent.K2_GetComponentLocation` _rollingball))
  (set `self.StartRotation` (`SceneComponent.K2_GetComponentRotation` _rollingball))
  (`PrimitiveComponent.SetSimulatePhysics` (`self.RollingBall`) false))

(event `self.ReceiveActorBeginOverlap`
  (params (OtherActor :type "Actor Object Reference")))

(event `Key|E` :consume false :overrideparent false
  (params (Key :type "Key Structure"))
  (bind _rollingball (`self.RollingBall`))
  (:`Pressed`
    (`self.ClearTrail` :!label _label)
    (`/Engine/EditorBlueprintResources/StandardMacros.DoOnce` false :!label _label_2
      (:`Completed`
        (`PrimitiveComponent.SetSimulatePhysics` _rollingball true)
        (`PrimitiveComponent.AddImpulse` _rollingball (0.0 15000.0 0.0) "None" false)
        (set `self.IsRolling` true)))))

(event `Key|T` :consume false :overrideparent false
  (params (Key :type "Key Structure"))
  (bind _rollingball (`self.RollingBall`))
  (:`Pressed`
    (set `self.IsRolling` false :!label _label_3)
    (`PrimitiveComponent.SetSimulatePhysics` _rollingball false)
    (`PrimitiveComponent.SetPhysicsLinearVelocity` _rollingball (0.0 0.0 0.0) false "None")
    (`SceneComponent.K2_SetWorldLocationAndRotation` _rollingball (`self.StartLocation`) (`self.StartRotation`) false false)
    (goto _label_2 :!via `Reset`)))

(event `StartRoll`
  (goto _label))

(event `EggReset`
  (goto _label_3))

(event `ClearTrail`)

(event `self.ReceiveTick`
  (params (DeltaSeconds :type "Float (single-precision)")))

(event `Key|N`
  (params (Key :type "Key Structure"))
  (:`Pressed`
    (`self.Damage`)))

(event `Damage`
  (bind _returnvalue (`GameplayStatics.GetPlayerController` 0))
  (`KismetSystemLibrary.PrintString` (`KismetStringLibrary.Conv_DoubleToString` (`self.Health`)))
  (bind _returnvalue_2 (`GameplayStatics.ApplyDamage` self 1.0))
  (set `self.Health` (- (`self.Health`) _returnvalue_2))
  (if (< (`self.Health`) 1.0)
    (`SceneComponent.SetVisibility` (`self.egg Shape`) false false)
    (`KismetSystemLibrary.PrintString` "dead")
    (`PrimitiveComponent.SetSimulatePhysics` (`self.RollingBall`) false)
    (bind _returnvalue_3 (`|CreateWidget` "/Game/UI/GameOverScreen.GameOverScreen_C"))
    (`UserWidget.AddToViewport` _returnvalue_3 0)
    (`WidgetBlueprintLibrary.SetInputMode_UIOnlyEx` _returnvalue _returnvalue_3)
    (set `PlayerController.bShowMouseCursor` true _returnvalue)
    (else
      (`KismetSystemLibrary.PrintString` "damaged")
      (if (== (`self.Health`) 2.0)
        (`PrimitiveComponent.SetMaterial` (`self.egg Shape`) 0 "/Game/StarterContent/Materials/M_Ground_Grass.M_Ground_Grass")
        (else
          (`PrimitiveComponent.SetMaterial` (`self.egg Shape`) 0 "/Game/StarterContent/Materials/M_Metal_Gold.M_Metal_Gold"))))))

(fn `UserConstructionScript`)