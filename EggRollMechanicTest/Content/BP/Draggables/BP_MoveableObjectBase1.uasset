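; BP_MoveableObjectBase1 is a moveable object base, filed under Draggables, that tracks whether it overlaps anything blocking.
; Its OverlapCheck component sets IsOverlapping when it begins overlapping a component tagged "Blocking".
; When such an overlap ends, it clears the flag and rescans the remaining overlaps, so the flag stays set while any blocker remains.
; The file contains no movement or drag logic.
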(event `self.OverlapCheck.OnComponentBeginOverlap`
  (params (OverlappedComponent :type "PrimitiveComponent Object Reference") (OtherActor :type "Actor Object Reference") (OtherComp :type "PrimitiveComponent Object Reference") (OtherBodyIndex :type Integer) (bFromSweep :type Boolean) (SweepResult :type "HitResult Structure (by ref)"))
  (if (`ActorComponent.ComponentHasTag` OtherComp "Blocking")
    (set `self.IsOverlapping` true)))

(event `self.OverlapCheck.OnComponentEndOverlap`
  (params (OverlappedComponent :type "PrimitiveComponent Object Reference") (OtherActor :type "Actor Object Reference") (OtherComp :type "PrimitiveComponent Object Reference") (OtherBodyIndex :type Integer))
  (if (`ActorComponent.ComponentHasTag` OtherComp "Blocking")
    (set `self.IsOverlapping` false)
    (for _array_element (`PrimitiveComponent.GetOverlappingComponents` (`self.OverlapCheck`))
      (if (`ActorComponent.ComponentHasTag` _array_element "Blocking")
        (set `self.IsOverlapping` true)))
    (if (`self.IsOverlapping`)
      _)))

(fn `UserConstructionScript`)