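; BP_StarObjective is a collectible star that adds to the BP_EggPlayer's Score when the player overlaps its sphere.
; On pickup it sets HasCleared, disables collision and plays a timeline that spins and shrinks the star to zero scale.
; ReloadStarsCheck restores a cleared star after a short delay by reversing that timeline, re-enabling collision and resetting the player's Score to zero.
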(event `self.ReceiveBeginPlay`
  (bind _returnvalue (`GameplayStatics.GetActorOfClass` "/Game/Egg/BP_EggPlayer.BP_EggPlayer_C"))
  (set `self.BP_EggPlayer` _returnvalue))

(event `self.Sphere.OnComponentBeginOverlap`
  (params (OverlappedComponent :type "PrimitiveComponent Object Reference") (OtherActor :type "Actor Object Reference") (OtherComp :type "PrimitiveComponent Object Reference") (OtherBodyIndex :type Integer) (bFromSweep :type Boolean) (SweepResult :type "HitResult Structure (by ref)"))
  (bind _bp_eggplayer (`self.BP_EggPlayer`))
  (bind _starplaceholder (`self.StarPlaceHolder`))
  ;[1 1 1] Spins and shrinks star if overlapped by marble, and marks as hidden
  (cast `/Game/Egg/BP_EggPlayer` OtherActor)
  (if (not (`self.HasCleared`))
    (bind _result (`/Engine/EditorBlueprintResources/StandardMacros.IncrementInt` (`/Game/Egg/BP_EggPlayer.Score` _bp_eggplayer))
      (:`  `
        (set `/Game/Egg/BP_EggPlayer.Score` _result _bp_eggplayer)
        (set `self.HasCleared` true)
        (`PrimitiveComponent.SetCollisionEnabled` (`self.Sphere`) "NoCollision")
        (bind (_direction _newtrack_0) (`Timeline|Timeline_0` :!via `PlayFromStart` :!label _label)
          (:`Update`
            (`SceneComponent.SetRelativeScale3D` _starplaceholder (`KismetMathLibrary.VLerp` (13.5 13.5 13.5) (0.0 0.0 0.0) _newtrack_0))
            (`SceneComponent.K2_SetRelativeRotation` _starplaceholder (`KismetMathLibrary.RLerp` (struct) (struct :`Yaw` -180.0) _newtrack_0) false false)))))))

(event `ReloadStarsCheck`
  ;[1 1 1] On Space bar re-set sets star to visable and plays spin animation
  (if (`self.HasCleared`)
    (`KismetSystemLibrary.Delay` 0.1)
    (set `self.HasCleared` false)
    (set `/Game/Egg/BP_EggPlayer.Score` 0 (`self.BP_EggPlayer`))
    (`SceneComponent.SetVisibility` (`self.StarPlaceHolder`) true false)
    (`PrimitiveComponent.SetCollisionEnabled` (`self.Sphere`) "QueryAndPhysics")
    (goto _label :!via `Reverse`)))

(fn `UserConstructionScript`)