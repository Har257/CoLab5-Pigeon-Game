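; Level gameplay manager that switches play between the rollable egg pawn and the edit camera pawn, and shows overlay and fail-screen widgets.
; Start/StopRoll, also bound to Space, resets the egg and reloads stars when a roll starts or stops.
; Timelines lerp the edit camera to the egg view before possession, or optionally back to its start.
; A SwappingMode flag blocks re-entry, and the GameInstance records the current mode.
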(event `Overlay menu`
  (bind _returnvalue (`|CreateWidget` "/Game/BP/UI/WBP_ScreenOverlay.WBP_ScreenOverlay_C" (`GameplayStatics.GetPlayerController` 0)))
  (`UserWidget.AddToViewport` _returnvalue 0)
  (`WidgetBlueprintLibrary.SetInputMode_GameAndUIEx` (`GameplayStatics.GetPlayerController` 0) _returnvalue "DoNotLock" false))

(event `EggDied`
  (bind _returnvalue (`GameplayStatics.GetPlayerController` 0))
  (bind _returnvalue_2 (`|CreateWidget` "/Game/BP/UI/WBP_FailScreen.WBP_FailScreen_C" (`GameplayStatics.GetPlayerController` 0)))
  (`UserWidget.AddToViewport` _returnvalue_2 0)
  (`WidgetBlueprintLibrary.SetInputMode_UIOnlyEx` _returnvalue _returnvalue_2)
  (set `PlayerController.bShowMouseCursor` true _returnvalue))

(event `EggPossess`
  (`Controller.Possess` (`GameplayStatics.GetPlayerController` 0) (`self.BP_EggPlayer`))
  (set `/Game/BP/BP_GIManager.IsInEggMode` true (`self.GameInstance`)))

(event `self.ReceiveBeginPlay`
  (bind _asbp_gimanager (cast `/Game/BP/BP_GIManager` (`GameplayStatics.GetGameInstance`)))
  (set `self.GameInstance` _asbp_gimanager)
  (bind _returnvalue (`GameplayStatics.GetActorOfClass` "/Game/Egg/BP_EggPlayer.BP_EggPlayer_C"))
  (set `self.BP_EggPlayer` _returnvalue)
  (bind _returnvalue_2 (`GameplayStatics.GetActorOfClass` "/Game/BP/BP_EditCamPlayer.BP_EditCamPlayer_C"))
  (set `self.BP_EditCam` _returnvalue_2)
  (bind _outactors (`GameplayStatics.GetAllActorsOfClass` "/Game/BP/BP_StarObjective.BP_StarObjective_C"))
  (set `self.AllLevelStars` _outactors)
  (set `self.EggCamDefultLocation` (`SceneComponent.K2_GetComponentLocation` (`/Game/Egg/BP_EggPlayer.EggCam` (`self.BP_EggPlayer`))))
  (set `self.EditCamDefultStartLocatiom` (`SceneComponent.K2_GetComponentLocation` (`/Game/BP/BP_EditCamPlayer.Camera` (`self.BP_EditCam`))))
  (`self.EnableInput` (`GameplayStatics.GetPlayerController` 0))
  (if (`self.StartEgg`)
    (`self.EggPossess`)
    (else
      (`self.EditCamPossess`))))

(event `EditCamPossess`
  (bind _returnvalue (`GameplayStatics.GetPlayerController` 0))
  (bind _bp_editcam (`self.BP_EditCam`))
  (`Controller.Possess` (`GameplayStatics.GetPlayerController` 0) _bp_editcam)
  (set `/Game/BP/BP_GIManager.IsInEggMode` false (`self.GameInstance`))
  (`self.EnableInput` _bp_editcam _returnvalue)
  (set `PlayerController.bShowMouseCursor` true _returnvalue))

(event `Start/StopRoll`
  (bind _bp_editcam (`self.BP_EditCam`))
  (bind _bp_editcam_2 (`self.BP_EditCam`))
  (bind _bp_eggplayer (`self.BP_EggPlayer`))
  (bind _rootcomponent (`Actor.RootComponent` (`self.BP_EditCam`)))
  (bind _returnvalue (`SceneComponent.K2_GetComponentLocation` (`/Game/Egg/BP_EggPlayer.EggCam` _bp_eggplayer)))
  (if (`self.SwappingMode`) :!label _label
    _
    (elif (`/Game/BP/BP_GIManager.IsInEggMode` (`self.GameInstance`))
      (set `self.SwappingMode` true)
      (if (`/Game/Egg/BP_EggPlayer.IsRolling` _bp_eggplayer)
        (`SceneComponent.K2_SetWorldLocation` _rootcomponent _returnvalue false false)
        (`/Game/Egg/BP_EggPlayer.EggReset` _bp_eggplayer)
        (`/Game/BP/BP_StarObjective.ReloadStarsCheck` (`self.AllLevelStars`))
        (else
          (`SceneComponent.K2_SetWorldLocation` _rootcomponent _returnvalue false false)))
      (if (`self.RetunEditCamToStartLocation`)
        (set `self.EditCamCurrentLocation` (`SceneComponent.K2_GetComponentLocation` (`/Game/BP/BP_EditCamPlayer.Camera` (`self.BP_EditCam`))))
        (`Controller.Possess` (`GameplayStatics.GetPlayerController` 0) _bp_editcam_2)
        (bind (_direction _editcamtoeggcam) (`Timeline|Timeline_0` :!via `PlayFromStart`)
          (:`Update`
            (`SceneComponent.K2_SetWorldLocation` (`Actor.RootComponent` _bp_editcam_2) (`KismetMathLibrary.VLerp` (`self.EditCamCurrentLocation`) (`self.EditCamDefultStartLocatiom`) _editcamtoeggcam) false false))
          (:`Finished`
            (`self.EditCamPossess`)
            (set `self.SwappingMode` false)))
        (else
          (`self.EditCamPossess`)
          (set `self.SwappingMode` false)))
      (else
        (`/Game/Egg/BP_EggPlayer.EggReset` (`self.BP_EggPlayer`))
        (`/Game/BP/BP_StarObjective.ReloadStarsCheck` (`self.AllLevelStars`))
        (set `self.SwappingMode` true)
        (`/Game/BP/BP_EditCamPlayer.Forced Drop` _bp_editcam)
        (`self.DisableInput` _bp_editcam null)
        (set `self.EditCamCurrentLocation` (`SceneComponent.K2_GetComponentLocation` (`/Game/BP/BP_EditCamPlayer.Camera` _bp_editcam)))
        (set `PlayerController.bShowMouseCursor` false (`GameplayStatics.GetPlayerController` 0))
        (bind (_direction_2 _editcamtoeggcam_2) (`Timeline|Timeline` :!via `PlayFromStart`)
          (:`Update`
            (`SceneComponent.K2_SetWorldLocation` (`Actor.RootComponent` (`self.BP_EditCam`)) (`KismetMathLibrary.VLerp` (`self.EditCamCurrentLocation`) (`self.EggCamDefultLocation`) _editcamtoeggcam_2) false false))
          (:`Finished`
            (`self.EggPossess`)
            (set `self.SwappingMode` false)))))))

(event `Key|SpaceBar` :consume false :overrideparent false
  (params (Key :type "Key Structure"))
  (:`Pressed`
    (goto _label)))

(fn `UserConstructionScript`)