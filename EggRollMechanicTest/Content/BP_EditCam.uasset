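; BP_EditCam is an edit-mode Blueprint for mouse-dragging BP_MoveableObjectBase actors.
; Left press selects the actor under the cursor; release realigns its OverlapCheck to its root and deselects.
; While selected, Tick grid-snaps the cursor hit on a fixed-X YZ plane, probes it with OverlapCheck, and moves the root there only if not overlapping.
; The input-enable and cursor-display nodes are unconnected.
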(event `self.ReceiveBeginPlay`)

(event `Key|LeftMouseButton` :consume false :overrideparent false
  (params (Key :type "Key Structure"))
  (:`Pressed`
    (bind _asbp_moveable_object_base (cast `/Game/BP_MoveableObjectBase` (`.HitActor` (`GameplayStatics.BreakHitResult` (`PlayerController.GetHitResultUnderCursorByChannel` (`GameplayStatics.GetPlayerController` 0) "TraceTypeQuery1" true)))))
    (bind _output_get (set `self.SelectedObject` _asbp_moveable_object_base))
    (set `self.ObjectSelected` true)
    (`KismetSystemLibrary.PrintString` (`KismetSystemLibrary.GetDisplayName` _output_get)))
  (:`Released`
    (`SceneComponent.K2_SetWorldLocation` (`/Game/BP_MoveableObjectBase.OverlapCheck` (`self.SelectedObject`)) (`SceneComponent.K2_GetComponentLocation` (`/Game/BP_MoveableObjectBase.DefaultSceneRoot` (`self.SelectedObject`))) false false)
    (set `self.ObjectSelected` false)
    (set `self.SelectedObject` null)))

(event `DraggingObject1`
  (bind _selectedobject (`self.SelectedObject`))
  (bind _output_get (set `self.TestLocation` (`KismetMathLibrary.MakeVector` 550.0 (`KismetMathLibrary.GridSnap_Float` (.y (`.ImpactPoint` (`GameplayStatics.BreakHitResult` (`PlayerController.GetHitResultUnderCursorByChannel` (`GameplayStatics.GetPlayerController` 0) "TraceTypeQuery1" true)))) 10.0) (`KismetMathLibrary.GridSnap_Float` (.z (`.ImpactPoint` (`GameplayStatics.BreakHitResult` (`PlayerController.GetHitResultUnderCursorByChannel` (`GameplayStatics.GetPlayerController` 0) "TraceTypeQuery1" true)))) 10.0))))
  (`SceneComponent.K2_SetWorldLocation` (`/Game/BP_MoveableObjectBase.OverlapCheck` _selectedobject) _output_get false false)
  (if (not (`/Game/BP_MoveableObjectBase.IsOverlapping` _selectedobject))
    (bind _output_get_2 (set `self.ViableLocation` (`self.TestLocation`)))
    (`SceneComponent.K2_SetWorldLocation` (`/Game/BP_MoveableObjectBase.OverlapCheck` (`self.SelectedObject`)) _output_get_2 false false)
    (`SceneComponent.K2_SetWorldLocation` (`/Game/BP_MoveableObjectBase.DefaultSceneRoot` (`self.SelectedObject`)) _output_get_2 false false)))

(event `self.ReceiveTick`
  (params (DeltaSeconds :type "Float (single-precision)"))
  (if (`self.ObjectSelected`)
    (`self.DraggingObject1`)))

(fn `UserConstructionScript`)