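; Edit-mode camera pawn for arranging BP_MoveableObjectBase actors with the mouse, handing control back to its instigator and destroying itself on T.
; Right-drag pans the camera and the wheel moves it along its view.
; Holding left-click drags the object under the cursor grid-snapped on a fixed-X plane, with the wheel rolling it in steps.
; Moves and rotations go to its OverlapCheck component first, reaching the object only when nothing overlaps.
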(event `Key|T`
  (params (Key :type "Key Structure"))
  (:`Pressed`
    (`KismetSystemLibrary.PrintString` "Edit mode Finished")
    (`Controller.Possess` (`GameplayStatics.GetPlayerController` 0) (`self.GetInstigator`))
    (`self.K2_DestroyActor`)))

(event `RotateToCheck`
  (bind _selectedobject (`self.SelectedObject`))
  (bind _rootcomponent (`Actor.RootComponent` _selectedobject))
  (if (not (`/Game/BP_MoveableObjectBase.IsOverlapping` (`self.SelectedObject`)))
    (`SceneComponent.K2_SetWorldRotation` _rootcomponent (`SceneComponent.K2_GetComponentRotation` (`/Game/BP_MoveableObjectBase.OverlapCheck` (`self.SelectedObject`))) false false)
    (`SceneComponent.K2_SetWorldRotation` (`/Game/BP_MoveableObjectBase.OverlapCheck` _selectedobject) (`SceneComponent.K2_GetComponentRotation` _rootcomponent) false false)
    (set `self.TryingRotate` false)))

(event `Key|MouseScrollUp` :consume false :overrideparent false
  (params (Key :type "Key Structure"))
  (:`Pressed`
    (if (`self.LmbHeld`)
      (if (`self.ObjectSelected`)
        (set `self.TryingRotate` true)
        (`SceneComponent.K2_SetWorldRotation` (`/Game/BP_MoveableObjectBase.OverlapCheck` (`self.SelectedObject`)) (`KismetMathLibrary.MakeRotator` (+ (.roll (`SceneComponent.K2_GetComponentRotation` (`/Game/BP_MoveableObjectBase.OverlapCheck` (`self.SelectedObject`)))) 45.0) (.pitch (`SceneComponent.K2_GetComponentRotation` (`/Game/BP_MoveableObjectBase.OverlapCheck` (`self.SelectedObject`)))) (.yaw (`SceneComponent.K2_GetComponentRotation` (`/Game/BP_MoveableObjectBase.OverlapCheck` (`self.SelectedObject`))))) false false)))))

(event `self.ReceiveBeginPlay`
  (bind _returnvalue (`GameplayStatics.GetPlayerController` 0))
  (`self.EnableInput` _returnvalue)
  (set `PlayerController.bShowMouseCursor` true _returnvalue))

(event `Key|MouseScrollDown` :consume false :overrideparent false
  (params (Key :type "Key Structure"))
  (:`Pressed`
    (if (`self.LmbHeld`)
      (if (`self.ObjectSelected`)
        (set `self.TryingRotate` true)
        (`SceneComponent.K2_SetWorldRotation` (`/Game/BP_MoveableObjectBase.OverlapCheck` (`self.SelectedObject`)) (`KismetMathLibrary.MakeRotator` (- (.roll (`SceneComponent.K2_GetComponentRotation` (`/Game/BP_MoveableObjectBase.OverlapCheck` (`self.SelectedObject`)))) 45.0) (.pitch (`SceneComponent.K2_GetComponentRotation` (`/Game/BP_MoveableObjectBase.OverlapCheck` (`self.SelectedObject`)))) (.yaw (`SceneComponent.K2_GetComponentRotation` (`/Game/BP_MoveableObjectBase.OverlapCheck` (`self.SelectedObject`))))) false false)))))

(event `Key|LeftMouseButton` :consume false :overrideparent false
  (params (Key :type "Key Structure"))
  (bind _defaultsceneroot (`/Game/BP_MoveableObjectBase.DefaultSceneRoot` (`self.SelectedObject`)))
  (:`Pressed`
    (set `self.LmbHeld` true)
    (bind _asbp_moveable_object_base (cast `/Game/BP_MoveableObjectBase` (`.HitActor` (`GameplayStatics.BreakHitResult` (`PlayerController.GetHitResultUnderCursorByChannel` (`GameplayStatics.GetPlayerController` 0) "TraceTypeQuery2" true)))))
    (set `self.SelectedObject` _asbp_moveable_object_base)
    (set `self.ObjectSelected` true))
  (:`Released`
    (set `self.LmbHeld` false)
    (if (`self.ObjectSelected`)
      (`SceneComponent.K2_SetWorldLocationAndRotation` (`/Game/BP_MoveableObjectBase.OverlapCheck` (`self.SelectedObject`)) (`SceneComponent.K2_GetComponentLocation` _defaultsceneroot) (`SceneComponent.K2_GetComponentRotation` _defaultsceneroot) false false)
      (set `self.ObjectSelected` false)
      (set `self.SelectedObject` null))))

(event `Key|MouseScrollUp` :consume false :overrideparent false
  (params (Key :type "Key Structure"))
  (:`Pressed`
    (if (not (`self.LmbHeld`))
      (`self.AddMovementInput` (`SceneComponent.GetForwardVector` (`self.Camera`))))))

(event `DraggingObject`
  (bind _selectedobject (`self.SelectedObject`))
  (bind _output_get (set `self.TestLocation` (`KismetMathLibrary.MakeVector` 550.0 (`KismetMathLibrary.GridSnap_Float` (.y (`.ImpactPoint` (`GameplayStatics.BreakHitResult` (`PlayerController.GetHitResultUnderCursorByChannel` (`GameplayStatics.GetPlayerController` 0) "TraceTypeQuery2" true)))) 10.0) (`KismetMathLibrary.GridSnap_Float` (.z (`.ImpactPoint` (`GameplayStatics.BreakHitResult` (`PlayerController.GetHitResultUnderCursorByChannel` (`GameplayStatics.GetPlayerController` 0) "TraceTypeQuery2" true)))) 10.0))))
  (`SceneComponent.K2_SetWorldLocation` (`/Game/BP_MoveableObjectBase.OverlapCheck` _selectedobject) _output_get false false)
  (if (not (`/Game/BP_MoveableObjectBase.IsOverlapping` _selectedobject))
    (bind _output_get_2 (set `self.ViableLocation` (`self.TestLocation`)))
    (`SceneComponent.K2_SetWorldLocation` (`/Game/BP_MoveableObjectBase.OverlapCheck` (`self.SelectedObject`)) _output_get_2 false false)
    (`SceneComponent.K2_SetWorldLocation` (`/Game/BP_MoveableObjectBase.DefaultSceneRoot` (`self.SelectedObject`)) _output_get_2 false false)))

(event `Key|MouseScrollDown` :consume false :overrideparent false
  (params (Key :type "Key Structure"))
  (:`Pressed`
    (if (not (`self.LmbHeld`))
      (`self.AddMovementInput` (* (`SceneComponent.GetForwardVector` (`self.Camera`)) -1)))))

(event `Key|RightMouseButton` :consume false :overrideparent false
  (params (Key :type "Key Structure"))
  (bind (_locationx _locationy) (`WidgetLayoutLibrary.GetMousePositionScaledByDPI` (`GameplayStatics.GetPlayerController` 0)))
  (:`Pressed`
    (set `self.MbDrag` true)
    (set `self.LastMousePos` (`KismetMathLibrary.MakeVector2D` _locationx _locationy)))
  (:`Released`
    (set `self.MbDrag` false)))

(event `self.ReceiveTick`
  (params (DeltaSeconds :type "Float (single-precision)"))
  (if (`self.MbDrag`)
    (`self.DragMoveUpdate`)
    (elif (`self.ObjectSelected`)
      (`self.DraggingObject`)
      (if (`self.TryingRotate`)
        (`self.RotateToCheck`)))))

(event `DragMoveUpdate`
  (bind (_locationx _locationy) (`WidgetLayoutLibrary.GetMousePositionScaledByDPI` (`GameplayStatics.GetPlayerController` 0)))
  (bind (_locationx_2 _locationy_2) (`WidgetLayoutLibrary.GetMousePositionScaledByDPI` (`GameplayStatics.GetPlayerController` 0)))
  (bind _returnvalue (`KismetMathLibrary.MakeVector2D` _locationx_2 _locationy_2))
  (`self.AddMovementInput` (`KismetMathLibrary.Normal` (`KismetMathLibrary.MakeVector` 0.0 (`KismetMathLibrary.BreakVector2D` (- (`self.LastMousePos`) _returnvalue)) (`.Y` (`KismetMathLibrary.BreakVector2D` (- _returnvalue (`self.LastMousePos`)))))) 0.5)
  (set `self.LastMousePos` (`KismetMathLibrary.MakeVector2D` _locationx _locationy)))

(fn `UserConstructionScript`)